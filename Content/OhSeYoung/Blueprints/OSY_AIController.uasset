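; AI controller that makes its controlled pawn chase the player character.
; Tick runs through a randomized Delay, so it periodically reissues a simple move toward player zero rather than every frame.
; A disconnected wander branch, which uses a forward line trace to choose between sidestepping right and moving ahead, never runs.
; A helper returning a random nearby destination is also unused.
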(event EventBeginPlay)

(event EventTick
  (params (DeltaSeconds :type Float%20%28single-precision%29))
  (Utilities|FlowControl|Delay (Math|Random|RandomFloatinRange 0.5 2.0))
  (AI|Navigation|SimpleMovetoActor self (Game|GetPlayerCharacter 0)))

(fn ConstructionScript)

(fn GetRandomDestination
  (return (+ (Transformation|GetActorLocation (Pawn|GetControlledPawn)) (Math|Vector|MakeVector (Math|Random|RandomFloatinRange -2.5e+02 2.5e+02) (Math|Random|RandomFloatinRange -2.5e+02 2.5e+02) 0.0))))